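; Player tank pawn Blueprint that wires input to aiming, track movement and firing.
; BeginPlay hands the barrel and turret components to the tank's aiming setters.
; Aim axes rotate an azimuth gimbal and spring arm at a frame-rate-independent rate to orbit the view.
; Throttle axes drive the left and right tracks independently, and the Fire action calls Fire.
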(event EventBeginPlay
  (Class|Tank|SetBarrelReference (Variables|Default|GetTankBarrel))
  (Class|Tank|SetTurretReference (Variables|Default|GetTankTurret)))

(event Input|ActionEvents|InputActionFire
  (params (Key :type Key%20Structure :default "AnyKey"))
  ;[1 1 1] Aim_Input_Bindings
  (:Pressed
    (Class|Tank|Fire)))

(event Input|AxisEvents|InputAxisRight_Track_Throttle
  (params (AxisValue :type Float%20%28single-precision%29))
  ;[1 1 1] Movement_Input_Bindings
  (Class|TankTrack|SetThrottle (Variables|Default|GetRightTrack) AxisValue))

(event Input|AxisEvents|InputAxisAimElevation
  (params (AxisValue :type Float%20%28single-precision%29))
  ;[1 1 1] Aim_Input_Bindings
  (Transformation|AddLocalRotation (Variables|Default|GetSpringArm) (Math|Rotator|MakeRotator 0.0 (* AxisValue (Utilities|Time|GetWorldDeltaSeconds) 1e+02) 0.0) false false))

(event Input|AxisEvents|InputAxisAimAzimuth
  (params (AxisValue :type Float%20%28single-precision%29))
  ;[1 1 1] Aim_Input_Bindings
  (Transformation|AddLocalRotation (Variables|Default|GetAzimuthGimbal) (Math|Rotator|MakeRotator 0.0 0.0 (* AxisValue (Utilities|Time|GetWorldDeltaSeconds) 1e+02)) false false))

(event Input|AxisEvents|InputAxisLeft_Track_Throttle
  (params (AxisValue :type Float%20%28single-precision%29))
  ;[1 1 1] Movement_Input_Bindings
  (Class|TankTrack|SetThrottle (Variables|Default|GetLeftTrack) AxisValue))

(fn ConstructionScript)